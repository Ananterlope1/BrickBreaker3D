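; Catapult character that previews a projectile trajectory and opens a settings UI at game start.
; BeginPlay adds a Setting_Widget to the viewport and switches player 0 to UI-only input.
; Tick runs a trace-channel projectile path prediction from LaunchPos, shown only through timed debug drawing.
; ForwardVelocity, LeftRightAngle and UpDownAngle feed the launch velocity's X, Y and Z directly, so the "angles" act as velocity components.
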(event `self.ReceiveBeginPlay`
  (bind _returnvalue (`|CreateWidget` "/Game/GameContent/Setting_Widget.Setting_Widget_C"))
  (`UserWidget.AddToViewport` _returnvalue 0)
  (`WidgetBlueprintLibrary.SetInputMode_UIOnlyEx` (`GameplayStatics.GetPlayerController` 0) null))

(event `self.ReceiveTick`
  (params (DeltaSeconds :type "Float (single-precision)"))
  (`GameplayStatics.Blueprint_PredictProjectilePath_ByTraceChannel` :`StartPos` (`SceneComponent.K2_GetComponentLocation` (`self.LaunchPos`)) :`LaunchVelocity` (`KismetMathLibrary.MakeVector` (`self.ForwardVelocity`) (`self.LeftRightAngle`) (`self.UpDownAngle`)) :`ProjectileRadius` 1.0 :`DrawDebugType` "ForDuration" :`DrawDebugTime` 1.0))

(fn `UserConstructionScript`)