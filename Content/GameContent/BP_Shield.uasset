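; BP_Shield is a destructible block that breaks after two strong impacts and adds to the player's BlocksDestroyed count on BP_CatapultChar.
; Box overlaps with a BP_Projectile pass the projectile's speed to DealDamage, while Cube hits pass the cube's own speed against a lower threshold.
; DealDamage counts impacts above the threshold: the first spawns an explosion and swaps to a damaged material, the second explodes and destroys the actor.
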(event `self.Box.OnComponentBeginOverlap`
  (params (OverlappedComponent :type "PrimitiveComponent Object Reference") (OtherActor :type "Actor Object Reference") (OtherComp :type "PrimitiveComponent Object Reference") (OtherBodyIndex :type Integer) (bFromSweep :type Boolean) (SweepResult :type "HitResult Structure (by ref)"))
  (bind _asbp_projectile (cast `/Game/GameContent/BP_Projectile` OtherActor))
  (`self.Deal Damage` (`KismetMathLibrary.VSize` (`SceneComponent.GetComponentVelocity` (`/Game/GameContent/BP_Projectile.StaticMesh` _asbp_projectile))) 1500.0))

(event `self.Cube.OnComponentHit`
  (params (HitComponent :type "PrimitiveComponent Object Reference") (OtherActor :type "Actor Object Reference") (OtherComp :type "PrimitiveComponent Object Reference") (NormalImpulse :type "Vector Structure") (Hit :type "HitResult Structure (by ref)"))
  (`self.Deal Damage` (`KismetMathLibrary.VSize` (`SceneComponent.GetComponentVelocity` (`self.Cube`))) 1000.0))

(fn `Deal Damage`
  (params (Velocity :type "Float (double-precision)") (`Velocity Threshold` :type "Float (double-precision)"))
  (bind _cube (`self.Cube`))
  (bind _returnvalue (`SceneComponent.K2_GetComponentLocation` _cube))
  (if (> Velocity `Velocity Threshold`)
    (bind _result (`/Engine/EditorBlueprintResources/StandardMacros.IncrementInt` (`self.IntSwitch`))
      (:`  `
        (switch `int` _result
          (:`1`
            (`GameplayStatics.SpawnEmitterAtLocation` "/Game/GameContent/P_Explosion.P_Explosion" _returnvalue)
            (`PrimitiveComponent.SetMaterial` _cube 0 "/Game/GameContent/M_Concrete_TilesDMG.M_Concrete_TilesDMG"))
          (:`2`
            (`GameplayStatics.SpawnEmitterAtLocation` "/Game/GameContent/P_Explosion.P_Explosion" _returnvalue)
            (`self.K2_DestroyActor`)
            (bind _asbp_catapult_char (cast `/Game/GameContent/BP_CatapultChar` (`GameplayStatics.GetPlayerCharacter` 0)))
            (bind _result_2 (`/Engine/EditorBlueprintResources/StandardMacros.IncrementInt` (`/Game/GameContent/BP_CatapultChar.BlocksDestroyed` _asbp_catapult_char))
              (:`  `
                (set `/Game/GameContent/BP_CatapultChar.BlocksDestroyed` _result_2 _asbp_catapult_char)))))))))

(fn `UserConstructionScript`)